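; Player controller that pans a PC_CameraPawn_BP through the MoveForward and MoveRight input axes.
; BeginPlay caches the controlled pawn, and each axis event sets its transform using the GetNewXTransform and GetNewYTransform helpers, which contain world X and Y offset math.
; CameraMoveSpeedCalc scales step size with the elevation spring arm's length, clamped to a range, so panning speeds up when zoomed out.
; Movement is unswept and not scaled by delta time.
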(event `self.ReceiveBeginPlay`
  (bind _aspc_camera_pawn_bp (cast `/Game/PC_Player/PC_CameraPawn_BP` (`self.K2_GetPawn`)))
  (set `self.CamRef` _aspc_camera_pawn_bp))

(event `InputAxis|MoveForward`
  (params (AxisValue :type "Float (single-precision)"))
  (bind _camref (`self.CamRef`))
  (`self.K2_SetActorTransform` _camref (`self.GetNewXTransform` _camref (`self.CameraMoveSpeedCalc`) AxisValue) false false))

(event `InputAxis|MoveRight`
  (params (AxisValue :type "Float (single-precision)"))
  (bind _camref (`self.CamRef`))
  (`self.K2_SetActorTransform` _camref (`self.GetNewYTransform` _camref (`self.CameraMoveSpeedCalc`) AxisValue) false false))

(fn `CameraMoveSpeedCalc`
  (returns (MoveSensitivity :type "Float (double-precision)"))
  (return (`KismetMathLibrary.FClamp` (/ (`SpringArmComponent.TargetArmLength` (`/Game/PC_Player/PC_CameraPawn_BP.ElevationRotationSpringArm` (`self.CamRef`))) 100.0) 5.0 20.0)))

(fn `UserConstructionScript`)