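; VR game mode that ends the game when a patrol guard perceives the player.
; On BeginPlay it finds every PatrolGuard in the level, stores them, and binds its OnSeePlayer handler to each guard's player-perceived event.
; When any guard fires that event, it adds the EndGameMenu_BP widget to the viewport, shows the mouse cursor and switches input to Game and UI focused on the menu.
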(event `self.ReceiveBeginPlay`
  (`self.GetGuardsAndRegisterListen` (delegate `OnSeePlayer`)))

(event `OnSeePlayer`
  (`self.ActivateEndgameUI`))

(fn `ActivateEndgameUI`
  (bind _returnvalue (`|CreateWidget` "/Game/UI/EndGameMenu_BP.EndGameMenu_BP_C"))
  (`UserWidget.AddToViewport` _returnvalue 0)
  (set `PlayerController.bShowMouseCursor` true (`GameplayStatics.GetPlayerController` 0))
  (`WidgetBlueprintLibrary.SetInputMode_GameAndUIEx` null _returnvalue "LockAlways" false))

(fn `GetGuardsAndRegisterListen`
  (params (Delegate :type "Delegate (by ref)"))
  (bind _outactors (`GameplayStatics.GetAllActorsOfClass` "/Game/PatrolGuard/Behavior/PatrolGuard.PatrolGuard_C"))
  (bind _output_get (set `self.Guards` _outactors))
  (for _array_element _output_get
    (add `PatrolGuard.OnPlayerPercieved` _array_element Delegate)))

(fn `UserConstructionScript`)