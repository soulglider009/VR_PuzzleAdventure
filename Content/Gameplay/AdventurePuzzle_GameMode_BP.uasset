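; Game mode for an adventure puzzle level that ends the game when a patrol guard touches the player.
; At BeginPlay it finds every PatrolGuard and binds its player-collision event to a handler that shows the endgame menu with the mouse cursor and game-and-UI input.
; It also spawns and possesses a motion controller pawn at the player start when a head-mounted display is enabled.
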(event `self.ReceiveBeginPlay`
  (`self.GetGuardsAndRegisterListen` (delegate `OnPlayerTouched`))
  (`self.SpawnPossesVRPawn` (`HeadMountedDisplayFunctionLibrary.IsHeadMountedDisplayEnabled`)))

(event `OnPlayerTouched`
  (`self.ActivateEndgameUI`))

(fn `ActivateEndgameUI`
  (bind _returnvalue (`|CreateWidget` "/Game/UI/EndGameMenu_BP.EndGameMenu_BP_C"))
  (`UserWidget.AddToViewport` _returnvalue 0)
  (set `PlayerController.bShowMouseCursor` true (`GameplayStatics.GetPlayerController` 0))
  (`WidgetBlueprintLibrary.SetInputMode_GameAndUIEx` null _returnvalue "LockAlways" false))

(fn `GetGuardsAndRegisterListen`
  (params (Delegate :type "Delegate (by ref)"))
  (bind _outactors (`GameplayStatics.GetAllActorsOfClass` "/Game/NPC/PatrolGuard/Behavior/PatrolGuard.PatrolGuard_C"))
  (bind _output_get (set `self.Guards` _outactors))
  (for _array_element _output_get
    (add `PatrolGuard.OnPlayerCollided` _array_element Delegate)))

(fn `SpawnPossesVRPawn`
  (params (bVROn :type Boolean))
  (bind _returnvalue (`GameplayStatics.GetPlayerController` 0))
  (if bVROn
    (bind _returnvalue_2 (`|SpawnActorFromClass` "/Game/Player/VRPawn/Blueprints/MotionControllerPawn.MotionControllerPawn_C" (`self.GetTransform` (`self.K2_FindPlayerStart` _returnvalue)) "AlwaysSpawn" "OverrideRootScale"))
    (`Controller.Possess` _returnvalue _returnvalue_2)))

(fn `UserConstructionScript`)