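; Adventure player controller that drives a separate Adventurer character and a free RTS-style camera pawn.
; Movement input moves the Adventurer relative to the camera yaw, or the headset camera in VR, and Jump is forwarded to it.
; The camera pawn edge-scrolls on Tick, yaws while RotateCamera is held, takes elevation input and can reset to an offset from the Adventurer.
; An old click-to-move path remains disconnected.
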(event `self.ReceiveBeginPlay`
  ;[1 1 1] Get ref to adventurer
  (set `self.AdventurerRef` (`self.GetAdventurerRef`))
  (set `self.ControlledPawn` (`self.K2_GetPawn`))
  (if (not (`HeadMountedDisplayFunctionLibrary.IsHeadMountedDisplayEnabled`))
    (`self.SetCameraStart`)))

(event `InputAxis|MoveForward`
  (params (AxisValue :type "Float (single-precision)"))
  (bind _returnvalue (`self.GetPawnRelativeRotation`))
  (bind _adventurerref (`self.AdventurerRef`))
  ;[1 1 1] WASD movement
  (`|ExecutionSequence` :!label _label
    (:`then_0`
      (`Pawn.AddMovementInput` _adventurerref (`KismetMathLibrary.GetForwardVector` _returnvalue) AxisValue false))
    (:`then_1`
      (`Pawn.AddMovementInput` _adventurerref (`KismetMathLibrary.GetRightVector` _returnvalue) (stale `InputAxis|MoveRight` AxisValue) false))))

(event `GameplaySetupFinished`
  ;[1 1 1] Gamemode calls, sets initial state
  (set `self.ControlledPawn` (`self.K2_GetPawn`)))

(event `InputAxis|MoveRight`
  (params (AxisValue :type "Float (single-precision)"))
  ;[1 1 1] WASD movement
  (goto _label))

(event `self.ReceiveTick`
  (params (DeltaSeconds :type "Float (single-precision)"))
  (`self.HandleMouseScroll`))

(event `InputAxis|CameraZUp`
  (params (AxisValue :type "Float (single-precision)"))
  ;[1 1 1] Q and E move camera elevation
  (`self.K2_SetActorTransform` (`self.ControlledPawn`) (`self.GetNewTransform` 0.0 0.0 AxisValue) false false))

(event `InputAxisKey|MouseX`
  (params (AxisValue :type "Float (single-precision)"))
  ;[1 1 1] Camera rotates (X only) when holding a key
  (`/Engine/EditorBlueprintResources/StandardMacros.Gate` true :!label _label_2
    (:`Exit`
      (`self.K2_SetActorRotation` (`self.ControlledPawn`) (`self.GetNewRotation` AxisValue) false))))

(event `InputAction|RotateCamera`
  (params (Key :type "Key Structure" :default "AnyKey"))
  ;[1 1 1] Camera rotates (X only) when holding a key
  (:`Pressed`
    (set `self.bCanRotate` true)
    (goto _label_2 :!via `Open`))
  (:`Released`
    (set `self.bCanRotate` false)
    (goto _label_2 :!via `Close`)))

(event `InputAction|ResetRTS`
  (params (Key :type "Key Structure" :default "AnyKey"))
  (:`Pressed`
    (`self.SetCameraStart`)))

(event `InputAction|Jump`
  (params (Key :type "Key Structure" :default "AnyKey"))
  (bind _adventurerref (`self.AdventurerRef`))
  (:`Pressed`
    (if (`Character.CanJump` _adventurerref)
      (`Character.Jump` _adventurerref))))

(fn `GetAdventurerRef`
  (returns (Adventurer :type "/Game/NPC/Adventurer/Behavior/Adventurer Object Reference"))
  (bind _outactors (`GameplayStatics.GetAllActorsOfClass` "/Game/NPC/Adventurer/Behavior/Adventurer.Adventurer_C"))
  (return (`KismetArrayLibrary.Array_Get` _outactors)))

(fn `GetNewRotation`
  (params (B :type "Float (double-precision)"))
  (returns (ReturnValue :type "Rotator Structure"))
  (bind (_returnvalue_roll _returnvalue_pitch _returnvalue_yaw) (`KismetMathLibrary.BreakRotator` (`self.K2_GetActorRotation` (`self.ControlledPawn`))))
  (return (`KismetMathLibrary.MakeRotator` _returnvalue_roll _returnvalue_pitch (+ _returnvalue_yaw (* (`self.PanSensitivity`) B)))))

(fn `GetPawnRefs`
  (set `self.ControlledPawn` (`self.K2_GetPawn`))
  (set `self.AdventurerRef` (`self.GetAdventurerRef`))
  (return))

(fn `GetPawnRelativeRotation`
  (returns (ReturnValue :type "Rotator Structure"))
  (locals (RotationToSEnd :type "Rotator Structure" :default (struct)))
  (`|ExecutionSequence`
    (:`then_0`
      (if (`HeadMountedDisplayFunctionLibrary.IsHeadMountedDisplayEnabled`)
        (bind _asmotion_controller_pawn (cast `/Game/Player/VRPawn/Blueprints/MotionControllerPawn` (`self.K2_GetPawn`)))
        (set `local.RotationToSEnd` (`SceneComponent.K2_GetComponentRotation` (`/Game/Player/VRPawn/Blueprints/MotionControllerPawn.Camera` _asmotion_controller_pawn)))
        (else
          (set `local.RotationToSEnd` (`KismetMathLibrary.MakeRotator` 0.0 0.0 (.yaw (`self.K2_GetActorRotation` (`self.ControlledPawn`))))))))
    (:`then_1`
      (return (`local.RotationToSEnd`)))))

(fn `GetXandYScroll`
  (returns (YScroll :type "Float (double-precision)") (XScroll :type "Float (double-precision)") (bYScroll :type Boolean) (bXScroll :type Boolean))
  (bind (_locationx _locationy) (`self.GetMousePosition`))
  (bind (_returnvalue_x _returnvalue_y) (`KismetMathLibrary.BreakVector2D` (`WidgetLayoutLibrary.GetViewportSize`)))
  (bind _returnvalue (- _locationx (/ _returnvalue_x 2.0)))
  (bind _returnvalue_2 (- (/ _returnvalue_y 2.0) _locationy))
  (return (`KismetMathLibrary.SignOfFloat` _returnvalue_2) (`KismetMathLibrary.SignOfFloat` _returnvalue) (>= (* (`KismetMathLibrary.Abs` _returnvalue_2) 2.0) (- _returnvalue_y (/ _returnvalue_y (`self.EdgeScrollDistance`)))) (>= (* (`KismetMathLibrary.Abs` _returnvalue) 2.0) (- _returnvalue_x (/ _returnvalue_x (`self.EdgeScrollDistance`))))))

(fn `HandleIfNeedToMove`
  (if (`self.bHasNewMove`)
    (`self.SendMoveToAdventurer` (`self.MoveToLocation`))))

(fn `HandleMouseScroll`
  (locals (ViewportX :type "Float (double-precision)") (ViewportY :type "Float (double-precision)") (bScroll :type Boolean))
  (bind (_yscroll _xscroll _byscroll _bxscroll) (`self.GetXandYScroll`))
  (bind _controlledpawn (`self.ControlledPawn`))
  (bind _controlledpawn_2 (`self.ControlledPawn`))
  (bind _mousesensitivity (`self.MouseSensitivity`))
  (bind _returnvalue (`self.K2_GetActorLocation` _controlledpawn))
  (`|ExecutionSequence`
    (:`then_0`
      (if _byscroll
        (`self.K2_SetActorLocation` _controlledpawn_2 (+ (* (`self.GetActorForwardVector` _controlledpawn) (* _yscroll _mousesensitivity)) _returnvalue) false false)))
    (:`then_1`
      (if _bxscroll
        (`self.K2_SetActorLocation` _controlledpawn_2 (+ _returnvalue (* (`self.GetActorRightVector` _controlledpawn) (* _mousesensitivity _xscroll))) false false)))))

(fn `HandleRTSSetMove`
  (bind (_hitresult _returnvalue) (`self.GetHitResultUnderCursorByChannel` "TraceTypeQuery2"))
  (if _returnvalue
    (set `self.bHasNewMove` true)
    (set `self.MoveToLocation` (`.Location` (`GameplayStatics.BreakHitResult` _hitresult)))
    (else
      (set `self.bHasNewMove` false))))

(fn `SendMoveToAdventurer`
  (params (MoveToLocation :type "Vector Structure")))

(fn `SetCameraStart`
  (`self.K2_SetActorLocation` (`self.ControlledPawn`) (+ (`self.K2_GetActorLocation` (`self.AdventurerRef`)) (`self.CameraOffsetStart`)) false false))

(fn `UserConstructionScript`)