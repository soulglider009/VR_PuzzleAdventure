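; RTS-style player controller that orders an AI-controlled adventurer around and drives the camera pawn, with a VR variant.
; While SetDestination is held, a gated Tick picks a destination by cursor trace, or by motion-controller line trace when an HMD is enabled.
; Releasing sends any valid hit to the adventurer's AI controller.
; Axis inputs set the pawn's transform, and holding RotateCamera lets MouseX yaw it.
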(event `self.ReceiveBeginPlay`
  (bind _returnvalue (`self.K2_GetPawn`))
  ;[1 1 1] Setup Camera and AI refs
  (bind _output_get (set `self.ControlledPawn` _returnvalue))
  (set `self.AdventurerAIControllerRef` (`self.GetAdventurerAIController`))
  (if (`HeadMountedDisplayFunctionLibrary.IsHeadMountedDisplayEnabled`)
    (`KismetSystemLibrary.PrintString` (`KismetSystemLibrary.GetDisplayName` (`self.ControlledPawn`)))
    (else
      (`self.K2_SetActorLocation` _output_get (+ (`self.K2_GetActorLocation` _returnvalue) (`self.CameraOffsetStart`)) false false))))

(event `self.ReceiveTick`
  (params (DeltaSeconds :type "Float (single-precision)"))
  (`/Engine/EditorBlueprintResources/StandardMacros.Gate` true :!label _label
    (:`Exit`
      (if (`HeadMountedDisplayFunctionLibrary.IsHeadMountedDisplayEnabled`)
        (`self.HandleVRSetMove`)
        (else
          (`self.HandleRTSSetMove`))))))

(event `InputAction|SetDestination`
  (params (Key :type "Key Structure" :default "AnyKey"))
  (:`Pressed`
    (set `self.bScanningToMove` false)
    (goto _label :!via `Open`))
  (:`Released`
    (`|ExecutionSequence`
      (:`then_0`
        (set `self.bScanningToMove` false)
        (goto _label :!via `Close`))
      (:`then_1`
        (if (`self.bHasNewMove`)
          (`self.SendMoveToAdventurer` (`self.MoveToLocation`)))))))

(event `InputAxis|MoveForward`
  (params (AxisValue :type "Float (single-precision)"))
  ;[1 1 1] Camera Movement
  (`self.K2_SetActorTransform` (`self.ControlledPawn`) (`self.GetNewTransform` AxisValue (stale `InputAxis|MoveRight` AxisValue) (stale `InputAxis|CameraZUp` AxisValue)) false false :!label _label_2))

(event `InputAxis|MoveRight`
  (params (AxisValue :type "Float (single-precision)"))
  ;[1 1 1] Camera Movement
  (goto _label_2))

(event `InputAxis|CameraZUp`
  (params (AxisValue :type "Float (single-precision)"))
  ;[1 1 1] Camera Movement
  (goto _label_2))

(event `InputAxisKey|MouseX`
  (params (AxisValue :type "Float (single-precision)"))
  ;[1 1 1] Camera rotates (X only) when holding a key
  (`/Engine/EditorBlueprintResources/StandardMacros.Gate` true :!label _label_3
    (:`Exit`
      (`self.K2_SetActorRotation` (`self.ControlledPawn`) (`self.GetNewRotation` AxisValue) false))))

(event `InputAction|RotateCamera`
  (params (Key :type "Key Structure" :default "AnyKey"))
  ;[1 1 1] Camera rotates (X only) when holding a key
  (:`Pressed`
    (set `self.bCanRotate` true)
    (goto _label_3 :!via `Open`))
  (:`Released`
    (set `self.bCanRotate` false)
    (goto _label_3 :!via `Close`)))

(fn `GetAdventurerAIController`
  (returns (`AsAdventurer AIController BP` :type "/Game/NPC/Adventurer/Behavior/Adventurer_AIController_BP Object Reference"))
  (bind _outactors (`GameplayStatics.GetAllActorsOfClass` "/Game/NPC/Adventurer/Behavior/Adventurer.Adventurer_C"))
  (bind _asadventurer_aicontroller_bp (cast `/Game/NPC/Adventurer/Behavior/Adventurer_AIController_BP` (`Pawn.GetController` (`KismetArrayLibrary.Array_Get` _outactors)))
    (:`then`
      _)
    (:`CastFailed`
      (`KismetSystemLibrary.PrintString` "Cast Fail Beginplay")))
  (return _asadventurer_aicontroller_bp))

(fn `GetNewRotation`
  (params (B :type "Float (double-precision)"))
  (returns (ReturnValue :type "Rotator Structure"))
  (bind (_returnvalue_roll _returnvalue_pitch _returnvalue_yaw) (`KismetMathLibrary.BreakRotator` (`self.K2_GetActorRotation` (`self.ControlledPawn`))))
  (return (`KismetMathLibrary.MakeRotator` _returnvalue_roll _returnvalue_pitch (+ _returnvalue_yaw (* (`self.PanSensitivity`) B)))))

(fn `HandleRTSSetMove`
  (bind (_hitresult _returnvalue) (`self.GetHitResultUnderCursorByChannel` "TraceTypeQuery2"))
  (if _returnvalue
    (set `self.bHasNewMove` true)
    (set `self.MoveToLocation` (`.Location` (`GameplayStatics.BreakHitResult` _hitresult)))
    (else
      (set `self.bHasNewMove` false))))

(fn `HandleVRSetMove`
  (bind _returnvalue (`self.GetComponentByClass` (`self.K2_GetPawn`) "/Script/HeadMountedDisplay.MotionControllerComponent"))
  (bind (_outhit _returnvalue_2) (`KismetSystemLibrary.LineTraceSingleForObjects` :`Start` (`SceneComponent.K2_GetComponentLocation` _returnvalue) :`End` (* (`SceneComponent.GetForwardVector` _returnvalue) (`self.LineTraceDistance`)) :`ObjectTypes` (`|MakeArray` "ObjectTypeQuery1" :!type "EObjectTypeQuery Enum") :`DrawDebugType` "ForOneFrame"))
  (if _returnvalue_2
    (set `self.bHasNewMove` true)
    (set `self.MoveToLocation` (`.ImpactPoint` (`GameplayStatics.BreakHitResult` _outhit)))
    (else
      (set `self.bHasNewMove` false))))

(fn `SendMoveToAdventurer`
  (params (MoveToLocation :type "Vector Structure"))
  (`/Game/NPC/Adventurer/Behavior/Adventurer_AIController_BP.Move To Event` (`self.AdventurerAIControllerRef`) MoveToLocation))

(fn `UserConstructionScript`)