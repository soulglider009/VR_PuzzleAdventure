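; Player controller for the RTS camera pawn that handles movement and yaw rotation input.
; Forward, right and vertical axis inputs share one SetActorTransform call fed by GetNewTransform, whose graph holds math for a sensitivity-scaled offset in pawn-local space.
; Holding RotateCamera opens a gate that lets MouseX change the pawn's yaw, scaled by PanSensitivity.
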(event `self.ReceiveBeginPlay`
  (set `self.CameraPawn` (`self.K2_GetPawn`)))

(event `InputAxis|MoveForward`
  (params (AxisValue :type "Float (single-precision)"))
  ;[1 1 1] Camera Movement
  (`self.K2_SetActorTransform` (`self.CameraPawn`) (`self.GetNewTransform` AxisValue (stale `InputAxis|MoveRight` AxisValue) (stale `InputAxis|CameraZUp` AxisValue)) false false :!label _label))

(event `InputAxis|MoveRight`
  (params (AxisValue :type "Float (single-precision)"))
  ;[1 1 1] Camera Movement
  (goto _label))

(event `InputAxis|CameraZUp`
  (params (AxisValue :type "Float (single-precision)"))
  ;[1 1 1] Camera Movement
  (goto _label))

(event `InputAxisKey|MouseX`
  (params (AxisValue :type "Float (single-precision)"))
  (bind (_returnvalue_roll _returnvalue_pitch _returnvalue_yaw) (`KismetMathLibrary.BreakRotator` (`self.K2_GetActorRotation` (`self.CameraPawn`))))
  (`/Engine/EditorBlueprintResources/StandardMacros.Gate` true :!label _label_2
    (:`Exit`
      (`self.K2_SetActorRotation` (`self.CameraPawn`) (`KismetMathLibrary.MakeRotator` _returnvalue_roll _returnvalue_pitch (+ _returnvalue_yaw (* (`self.PanSensitivity`) AxisValue))) false))))

(event `InputAction|RotateCamera`
  (params (Key :type "Key Structure" :default "AnyKey"))
  (:`Pressed`
    (set `self.bCanRotate` true)
    (goto _label_2 :!via `Open`))
  (:`Released`
    (set `self.bCanRotate` false)
    (goto _label_2 :!via `Close`)))

(fn `UserConstructionScript`)