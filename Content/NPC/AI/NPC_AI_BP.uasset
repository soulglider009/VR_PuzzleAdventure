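; AI controller for guard NPCs that starts the GuardBehavior tree with the GuardData blackboard on BeginPlay.
; Perception updates write sensed actors tagged "enemy" to the blackboard's enemy key and clear it when sensing fails.
; Two helpers go uncalled here: a perception debug print, and SetFocalPoint, which despite its name writes the player pawn to the enemy key.
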(event `self.ReceiveBeginPlay`
  (bind _blackboardcomponent (`self.UseBlackboard` "/Game/NPC/AI/GuardData.GuardData"))
  (`self.RunBehaviorTree` "/Game/NPC/AI/GuardBehavior.GuardBehavior")
  (set `self.BlackboardComp` _blackboardcomponent))

(event `self.AIPerception.OnTargetPerceptionUpdated`
  (params (Actor :type "Actor Object Reference") (Stimulus :type "AIStimulus Structure"))
  (bind _enemykey (`self.EnemyKey`))
  (if (`self.ActorHasTag` Actor "enemy")
    (if (`.bSuccessfullySensed` (break `AIStimulus` Stimulus))
      (`BlackboardComponent.SetValueAsObject` (`self.BlackboardComp`) (`KismetSystemLibrary.MakeLiteralName` _enemykey) Actor)
      (else
        (`BlackboardComponent.ClearValue` (`self.BlackboardComp`) _enemykey)))))

(fn `Print perception`
  (params (Object :type "Object Object Reference") (Stimulus :type "AIStimulus Structure (by ref)"))
  (bind _returnvalue (`AIPerceptionSystem.GetSenseClassForStimulus` Stimulus))
  (`KismetSystemLibrary.PrintString` (`KismetStringLibrary.Concat_StrStr` (`KismetSystemLibrary.GetObjectName` (`self.K2_GetPawn`)) " " (`KismetSystemLibrary.GetClassDisplayName` _returnvalue) " " (`KismetSystemLibrary.GetObjectName` Object))))

(fn `Set Focal Point`
  (params (Blackboard :type "BlackboardComponent Object Reference"))
  (`BlackboardComponent.SetValueAsObject` Blackboard (`KismetSystemLibrary.MakeLiteralName` (`self.EnemyKey`)) (`GameplayStatics.GetPlayerPawn` 0)))

(fn `UserConstructionScript`)