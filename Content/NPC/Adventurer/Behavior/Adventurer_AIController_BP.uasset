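; AI controller for the Adventurer NPC that drives it through a behavior tree and blackboard.
; On BeginPlay it runs the Adventurer behavior tree and caches the Adventurer blackboard component.
; A MoveTo event writes a target location to the blackboard's move-to key, printing the destination on screen for debugging.
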(event `self.ReceiveBeginPlay`
  (`self.RunBehaviorTree` "/Game/NPC/Adventurer/AI/AdventurerBehavior.AdventurerBehavior")
  (bind _blackboardcomponent (`self.UseBlackboard` "/Game/NPC/Adventurer/AI/AdventurerBlackboard.AdventurerBlackboard"))
  (set `self.BlackboardRef` _blackboardcomponent))

(event `Move To Event`
  (params (Location :type "Vector Structure"))
  (`self.Debug Move To Print` Location)
  (`BlackboardComponent.SetValueAsVector` (`self.BlackboardRef`) (`self.MoveToKey`) Location))

(fn `Debug Move To Print`
  (params (InVec :type "Vector Structure"))
  (`KismetSystemLibrary.PrintString` "Adventurer told to move to: " true true (struct :`G` 0.66 :`B` 1.0 :`A` 1.0) 5.0)
  (`KismetSystemLibrary.PrintString` (`KismetStringLibrary.Conv_VectorToString` InVec)))

(fn `UserConstructionScript`)